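; Puzzle character Blueprint that handles jumping and shows or hides an animated selection cursor widget.
; EnableSelectionWidget reveals the SelectionCursor widget component and loops its SelectionIcon cursor animation indefinitely.
; DisableSelectionWidget stops that animation and hides the component, and runs on BeginPlay so the cursor starts hidden.
; Nothing in this Blueprint calls EnableSelectionWidget.
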(event `self.ReceiveBeginPlay`
  (`self.DisableSelectionWidget`))

(event `InputAction|Jump`
  (params (Key :type "Key Structure"))
  (:`Pressed`
    (`self.Jump`)))

(fn `DisableSelectionWidget`
  (bind _asselection_icon (cast `/Game/HUD/SelectionIcon` (`WidgetComponent.GetUserWidgetObject` (`self.SelectionCursor`))))
  (`UserWidget.StopAnimation` _asselection_icon (`/Game/HUD/SelectionIcon.CursorAnimation` _asselection_icon))
  (`SceneComponent.SetVisibility` (`self.SelectionCursor`) false false))

(fn `EnableSelectionWidget`
  (bind _returnvalue (`WidgetComponent.GetUserWidgetObject` (`self.SelectionCursor`)))
  (bind _asselection_icon (cast `/Game/HUD/SelectionIcon` _returnvalue))
  (`UserWidget.PlayAnimation` _returnvalue (`/Game/HUD/SelectionIcon.CursorAnimation` _asselection_icon) 0.0 0 "Forward" 1.0 false)
  (`SceneComponent.SetVisibility` (`self.SelectionCursor`) true false))

(fn `UserConstructionScript`)