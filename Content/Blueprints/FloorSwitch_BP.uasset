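; Floor pressure switch that puzzle characters trigger by standing on it to activate and deactivate linked actors.
; An overlap box tracks characters; the first to enter sends ActivateMessage to AffectedActors implementing SwitchInterface_BP, plays a sound and moves the mesh vertically via a timeline.
; When the last leaves, it sends DeactivateMessage and reverses the timeline, unless StayActive is set to latch it on.
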(event `self.ReceiveBeginPlay`
  (set `self.InitialSwitchLocation` (`SceneComponent.K2_GetComponentLocation` (`self.SwitchMesh`))))

(event `self.Box.OnComponentBeginOverlap`
  (params (OverlappedComponent :type "PrimitiveComponent Object Reference") (OtherActor :type "Actor Object Reference") (OtherComp :type "PrimitiveComponent Object Reference") (OtherBodyIndex :type Integer) (bFromSweep :type Boolean) (SweepResult :type "HitResult Structure (by ref)"))
  (bind _characters (`self.Characters`))
  (bind _aspuzzle_character_bp (cast `/Game/Blueprints/Character/PuzzleCharacter_BP` OtherActor))
  (`KismetArrayLibrary.Array_Add` _characters _aspuzzle_character_bp)
  (if (== (`KismetArrayLibrary.Array_Length` _characters) 1)
    (for _array_element (`self.AffectedActors`)
      (if (`KismetSystemLibrary.DoesImplementInterface` _array_element "/Game/Blueprints/SwitchInterface_BP.SwitchInterface_BP_C")
        (message `/Game/Blueprints/SwitchInterface_BP.Activate` _array_element)))
    (`GameplayStatics.PlaySound2D` (`self.SwitchSound`) 1.0 1.0 0.0 null null)
    (bind (_direction _switchelevation) (`Timeline|SwitchTimeline` :!label _label)
      (:`Update`
        (`SceneComponent.K2_SetWorldLocation` (`self.SwitchMesh`) (`KismetMathLibrary.MakeVector` (.x (`self.InitialSwitchLocation`)) (.y (`self.InitialSwitchLocation`)) (+ _switchelevation (.z (`self.InitialSwitchLocation`)))) false false)))))

(event `self.Box.OnComponentEndOverlap`
  (params (OverlappedComponent :type "PrimitiveComponent Object Reference") (OtherActor :type "Actor Object Reference") (OtherComp :type "PrimitiveComponent Object Reference") (OtherBodyIndex :type Integer))
  (bind _aspuzzle_character_bp (cast `/Game/Blueprints/Character/PuzzleCharacter_BP` OtherActor))
  (if (not (`self.StayActive`))
    (`KismetArrayLibrary.Array_RemoveItem` (`self.Characters`) _aspuzzle_character_bp)
    (if (== (`KismetArrayLibrary.Array_Length` (`self.Characters`)) 0)
      (for _array_element (`self.AffectedActors`)
        (if (`KismetSystemLibrary.DoesImplementInterface` _array_element "/Game/Blueprints/SwitchInterface_BP.SwitchInterface_BP_C")
          (message `/Game/Blueprints/SwitchInterface_BP.Deactivate` _array_element)))
      (goto _label :!via `Reverse`))))

(fn `UserConstructionScript`)