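; Switch-driven statue that raises and turns its Fountain component, acting like a door that opens once enough switches are active.
; Activate and Deactivate adjust a switch count that is compared against SwitchRequirement.
; Reaching the requirement plays DoorTimeline, which offsets the Fountain's height and yaw from the transform cached at BeginPlay.
; Dropping below it reverses the timeline unless StayOpen is set.
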(event `self.ReceiveBeginPlay`
  (set `self.InitialDoorLocation` (`SceneComponent.K2_GetComponentLocation` (`self.Fountain`)))
  (set `self.InitialRotation` (`SceneComponent.K2_GetComponentRotation` (`self.Fountain`))))

(event `/Game/Blueprints/SwitchInterface_BP.Activate`
  (`/Engine/EditorBlueprintResources/StandardMacros.IncrementInt` (`self.SwitchesActivated`)
    (:`  `
      (if (>= (`self.SwitchesActivated`) (`self.SwitchRequirement`))
        (bind (_direction _doorelevation _statuerotation) (`Timeline|DoorTimeline` :!label _label)
          (:`Update`
            (`SceneComponent.K2_SetWorldLocationAndRotation` (`self.Fountain`) (`KismetMathLibrary.MakeVector` (.x (`self.InitialDoorLocation`)) (.y (`self.InitialDoorLocation`)) (+ _doorelevation (.z (`self.InitialDoorLocation`)))) (`KismetMathLibrary.MakeRotator` (.roll (`self.InitialRotation`)) (.pitch (`self.InitialRotation`)) (+ (.yaw (`self.InitialRotation`)) _statuerotation)) false false)))))))

(event `/Game/Blueprints/SwitchInterface_BP.Deactivate`
  (`/Engine/EditorBlueprintResources/StandardMacros.DecrementInt` (`self.SwitchesActivated`)
    (:`  `
      (if (< (`self.SwitchesActivated`) (`self.SwitchRequirement`))
        (if (not (`self.StayOpen`))
          (goto _label :!via `Reverse`))))))

(fn `UserConstructionScript`)