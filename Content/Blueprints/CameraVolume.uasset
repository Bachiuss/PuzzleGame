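; Camera volume that becomes the player's view target, with a cubic blend, when the puzzle character overlaps its box.
; On overlap it registers itself as the current camera volume on both the character and the puzzle player controller.
; When spline mode is on, Tick eases its camera toward the spline point closest to the character while smoothly rotating to look at them.
; BeginPlay caches the initial camera transform and spline setting.
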(event `self.ReceiveBeginPlay`
  (set `self.Controller` (`GameplayStatics.GetPlayerController` 0))
  (set `self.TurnUseSplineBackOn` (`self.UseSpline`))
  (set `self.InitialCameraTransform` (`SceneComponent.K2_GetComponentToWorld` (`self.Camera`))))

(event `self.Box.OnComponentBeginOverlap`
  (params (OverlappedComponent :type "PrimitiveComponent Object Reference") (OtherActor :type "Actor Object Reference") (OtherComp :type "PrimitiveComponent Object Reference") (OtherBodyIndex :type Integer) (bFromSweep :type Boolean) (SweepResult :type "HitResult Structure (by ref)"))
  (bind _aspuzzle_character_bp (cast `/Game/Blueprints/Character/PuzzleCharacter_BP` OtherActor))
  (bind _output_get (set `self.Character` _aspuzzle_character_bp))
  (set `/Game/Blueprints/Character/PuzzleCharacter_BP.CurrentCameraVolume` self _output_get)
  (`/Engine/EditorBlueprintResources/StandardMacros.IsValid` (`self.Controller`)
    (:`Is Valid`
      (bind _aspuzzle_player_controller_bp (cast `/Game/Blueprints/PuzzlePlayerController_BP` (`self.Controller`)))
      (set `/Game/Blueprints/PuzzlePlayerController_BP.CurrentCameraVolume` self _aspuzzle_player_controller_bp)
      (`PlayerController.SetViewTargetWithBlend` (`self.Controller`) self 2.0 "VTBlend_Cubic" 5.0 true))))

(event `self.ReceiveTick`
  (params (DeltaSeconds :type "Float (single-precision)"))
  (bind _camera (`self.Camera`))
  (bind _returnvalue (`self.K2_GetActorLocation` (`self.Character`)))
  (set `self.Delta Time` DeltaSeconds)
  (if (`self.UseSpline`)
    (`/Engine/EditorBlueprintResources/StandardMacros.IsValid` (`self.Character`)
      (:`Is Valid`
        (`SceneComponent.K2_SetWorldLocationAndRotation` (`self.Camera`) (`KismetMathLibrary.VInterpTo` (`SceneComponent.K2_GetComponentLocation` _camera) (`SplineComponent.FindLocationClosestToWorldLocation` (`self.Spline`) _returnvalue "World") (`self.Delta Time`) 2.0) (`KismetMathLibrary.RInterpTo` (`SceneComponent.K2_GetComponentRotation` _camera) (`KismetMathLibrary.FindLookAtRotation` (`SceneComponent.K2_GetComponentLocation` (`self.Camera`)) _returnvalue) (`self.Delta Time`) 2.0) false false)))))

(fn `UserConstructionScript`)